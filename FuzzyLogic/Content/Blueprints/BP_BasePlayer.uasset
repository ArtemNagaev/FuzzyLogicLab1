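; Player actor that runs an automatic duel against a simulated enemy, with random HP and strength stats and Paper2D flipbooks for both fighters.
; A looping one-second timer calls CheckTactic, which uses fuzzy membership functions to rate player HP and strength, each relative to enemy HP, as low/med/high.
; A rule table then picks Attack, Block or Run, which update HP and fighter modes.
; Tick applies those modes as animations and prints debug stats.
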(event Custom|RefreshAnimation)

(event EventBeginPlay
  (Utilities|FlowControl|Sequence
    (:then_0
      (bind _output_get (Variables|Default|SetHP_Player (Math|Random|RandomFloatinRange 5e+01 1e+02)))
      (Variables|Default|SetHP_PlayerInit _output_get)
      (Variables|Default|SetStrength_Player (Math|Random|RandomFloatinRange 5e+01 1e+02))
      (bind _output_get_2 (Variables|Default|SetHP_Enemy (Math|Random|RandomFloatinRange 5e+01 1e+02)))
      (Variables|Default|SetHP_EnemyInit _output_get_2)
      (Variables|Default|SetStrength_Enemy (Math|Random|RandomFloatinRange 5e+01 1e+02)))
    (:then_1
      (Utilities|Time|SetTimerbyFunctionName self "CheckTactic" 1.0 true))))

(event Collision|EventActorBeginOverlap
  (params (OtherActor :type Actor%20Object%20Reference)))

(event EventTick
  (params (DeltaSeconds :type Float%20%28single-precision%29))
  (Development|PrintText (Utilities|Text|FormatText "{1} HP Player 
{2} HP Enemy 
{3} Сoefficient 
{4} Player State" (Variables|Default|GetHP_Player) (Variables|Default|GetHP_Enemy) (/ (Variables|Default|GetHP_Player) (Variables|Default|GetHP_Enemy))) true true "(R=0.000000,G=0.660000,B=1.000000,A=1.000000)" 0.0)
  (CallFunction|SetAnimationPlayer (Variables|Default|GetPlayerMode))
  (CallFunction|SetAnimationEnemy (Variables|Default|GetEnemyMode)))

(fn ConstructionScript)

(fn Fuzzyand
  (params (A :type Float%20%28single-precision%29) (B :type Float%20%28single-precision%29))
  (return (Math|Float|Min(Float) A B)))

(fn Fuzzyor
  (params (A :type Float%20%28single-precision%29) (B :type Float%20%28single-precision%29))
  (return (Math|Float|Max(Float) A B)))

(fn FuzzyNot
  (params (A :type Float%20%28single-precision%29))
  (return (- 1.0 A)))

(fn CheckTactic
  (bind _hp_enemy (Variables|Default|GetHP_Enemy))
  (bind _hp_player (Variables|Default|GetHP_Player))
  (bind _hp_enemy_2 (Variables|Default|GetHP_Enemy))
  (bind _strength_player (Variables|Default|GetStrength_Player))
  (bind _returnvalue (/ _hp_player _hp_enemy_2))
  (bind _returnvalue_2 (/ _strength_player _hp_enemy))
  (Utilities|FlowControl|Sequence
    (:then_0
      (if (> _hp_enemy_2 0.0)
        (bind _functionvalue (CallFunction|MembershipFunction _returnvalue (Utilities|Array|MakeArray (Utilities|Struct|MakeSector 0.0 0.0 1.0 1.0) (Utilities|Struct|MakeSector 0.0 0.4 1.0 1.0) (Utilities|Struct|MakeSector 0.4 2.0 1.0 0.0))))
        (bind _functionvalue_2 (CallFunction|MembershipFunction _returnvalue (Utilities|Array|MakeArray (Utilities|Struct|MakeSector 0.0 0.8 0.0 1.0) (Utilities|Struct|MakeSector 0.8 1.2 1.0 1.0) (Utilities|Struct|MakeSector 1.2 2.0 1.0 0.0))))
        (bind _functionvalue_3 (CallFunction|MembershipFunction _returnvalue (Utilities|Array|MakeArray (Utilities|Struct|MakeSector 0.0 1.6 0.0 1.0) (Utilities|Struct|MakeSector 1.6 2.0 1.0 1.0) (Utilities|Struct|MakeSector 2.0 2.0 1.0 1.0))))
        (bind _newparam1 (CallFunction|GetLinguisticDescription (Utilities|Array|MakeArray (Utilities|Struct|MakeLinguisticDescriptionValue _functionvalue "low") (Utilities|Struct|MakeLinguisticDescriptionValue _functionvalue_2 "med") (Utilities|Struct|MakeLinguisticDescriptionValue _functionvalue_3 "high"))))
        (Variables|Default|SetHpCheck _newparam1)))
    (:then_1
      (if (> _hp_enemy 0.0)
        (bind _functionvalue_4 (CallFunction|MembershipFunction _returnvalue_2 (Utilities|Array|MakeArray (Utilities|Struct|MakeSector 0.0 0.0 1.0 1.0) (Utilities|Struct|MakeSector 0.0 0.4 1.0 1.0) (Utilities|Struct|MakeSector 0.4 2.0 1.0 0.0))))
        (bind _functionvalue_5 (CallFunction|MembershipFunction _returnvalue_2 (Utilities|Array|MakeArray (Utilities|Struct|MakeSector 0.0 0.8 0.0 1.0) (Utilities|Struct|MakeSector 0.8 1.2 1.0 1.0) (Utilities|Struct|MakeSector 1.2 2.0 1.0 0.0))))
        (bind _functionvalue_6 (CallFunction|MembershipFunction _returnvalue_2 (Utilities|Array|MakeArray (Utilities|Struct|MakeSector 0.0 1.6 0.0 1.0) (Utilities|Struct|MakeSector 1.6 2.0 1.0 1.0) (Utilities|Struct|MakeSector 2.0 2.0 1.0 1.0))))
        (bind _newparam1_2 (CallFunction|GetLinguisticDescription (Utilities|Array|MakeArray (Utilities|Struct|MakeLinguisticDescriptionValue _functionvalue_4 "low") (Utilities|Struct|MakeLinguisticDescriptionValue _functionvalue_5 "med") (Utilities|Struct|MakeLinguisticDescriptionValue _functionvalue_6 "high"))))
        (Variables|Default|SetStrCheck _newparam1_2)))
    (:then_2
      (switch string (Variables|Default|GetHpCheck)
        (:low
          (switch string (Variables|Default|GetStrCheck)
            (:low
              _)
            (:med
              _)
            (:high
              _))
          (CallFunction|Run))
        (:med
          (switch string (Variables|Default|GetStrCheck)
            (:low
              (CallFunction|Block))
            (:med
              (CallFunction|Block))
            (:high
              (CallFunction|Attack))))
        (:high
          (switch string (Variables|Default|GetStrCheck)
            (:low
              (CallFunction|Block))
            (:med
              (CallFunction|Attack))
            (:high
              (CallFunction|Attack))))))))

(fn MembershipFunction(depricated)
  (params (Value :type Float%20%28single-precision%29) (FirstSectorStart :type Float%20%28single-precision%29) (FirstSectorEnd :type Float%20%28single-precision%29) (SecondSectorStart :type Float%20%28single-precision%29) (SecondSectorEnd :type Float%20%28single-precision%29) (ThirdSectorStart :type Float%20%28single-precision%29) (ThirdSectorEnd :type Float%20%28single-precision%29) (MemberFirstStart :type Float%20%28single-precision%29) (MemberFirstEnd :type Float%20%28single-precision%29) (MemberSecondStart :type Float%20%28single-precision%29) (MemberSecondEnd :type Float%20%28single-precision%29) (MemberThirdStart :type Float%20%28single-precision%29) (MemberThirdEnd :type Float%20%28single-precision%29))
  (bind _returnvalue (Math|Float|MapRangeClamped Value FirstSectorStart FirstSectorEnd MemberFirstStart MemberFirstEnd))
  (bind _returnvalue_2 (Math|Float|MapRangeClamped Value SecondSectorStart SecondSectorEnd MemberSecondStart MemberSecondEnd))
  (bind _returnvalue_3 (Math|Float|MapRangeClamped Value ThirdSectorStart ThirdSectorEnd MemberThirdStart MemberThirdEnd))
  (if (< Value FirstSectorEnd)
    (Development|PrintString (Utilities|String|ToString(Float) _returnvalue))
    (return _returnvalue)
    (elif (< Value SecondSectorEnd)
      (Development|PrintString (Utilities|String|ToString(Float) _returnvalue_2))
      (return _returnvalue_2)
      (else
        (Development|PrintString (Utilities|String|ToString(Float) _returnvalue_3))
        (return _returnvalue_3)))))

(fn MembershipFunction
  (params (Value :type Float%20%28single-precision%29) (Sectors :type Array%20of%20Sector%20Structures))
  (bind _returnvalue (Utilities|Array|LastIndex Sectors))
  (bind _output (Utilities|Array|Get(acopy) Sectors))
  (bind _output_2 (Utilities|Array|Get(acopy) Sectors _returnvalue))
  (LocalVariables|SetValueLocal Value)
  (for _array_element Sectors
    (LocalVariables|SetSectorLocal _array_element)
    (if (and (>= (LocalVariables|GetValueLocal) (.x1 (LocalVariables|GetSectorLocal))) (< (LocalVariables|GetValueLocal) (.x2 (LocalVariables|GetSectorLocal))))
      (return (Math|Float|MapRangeClamped (LocalVariables|GetValueLocal) (.x1 (LocalVariables|GetSectorLocal)) (.x2 (LocalVariables|GetSectorLocal)) (.valuestart (LocalVariables|GetSectorLocal)) (.valueend (LocalVariables|GetSectorLocal))))))
  (if (<= (LocalVariables|GetValueLocal) (.x1 _output))
    (return (.valuestart _output))
    (elif (>= (LocalVariables|GetValueLocal) (.x2 _output_2))
      (return (.valueend _output_2))
      (else
        (return 0.0)))))

(fn GetLinguisticDescription
  (params (NewParam :type Array%20of%20Linguistic%20Description%20Value%20Structures))
  (bind _localmap (LocalVariables|GetLocalMap))
  (bind _output_get (LocalVariables|SetLocalArray NewParam))
  (for _array_element _output_get
    (Utilities|Map|Add (LocalVariables|GetLocalMap) (.memberfunctionvalue _array_element) (.linguisticdescription _array_element)))
  (bind _keys (Utilities|Map|Keys _localmap))
  (return (.Value (Utilities|Map|Find _localmap (.MaxValue (Math|Float|MaxOfFloatArray _keys))))))

(fn Attack
  (Development|PrintString "ATTACK" true true "(R=0.000000,G=0.660000,B=1.000000,A=1.000000)" 1.0)
  (Variables|Default|SetEnemyMode "NewEnumerator1")
  (Variables|Default|SetPlayerMode "NewEnumerator1")
  (bind _output_get (Variables|Default|SetHP_Enemy (- (Variables|Default|GetHP_Enemy) (Variables|Default|GetStrength_Player))))
  (if (<= _output_get 0.0)
    (Variables|Default|SetEnemyMode "NewEnumerator3")
    (Variables|Default|SetHP_Enemy (Math|Random|RandomFloatinRange 5e+01 1e+02))
    (else
      (bind _output_get_2 (Variables|Default|SetHP_Player (- (Variables|Default|GetHP_Player) (Variables|Default|GetStrength_Player))))
      (if (<= _output_get_2 0.0)
        (Variables|Default|SetPlayerMode "NewEnumerator3")
        (Variables|Default|SetHP_Player (Math|Random|RandomFloatinRange 5e+01 1e+02))))))

(fn Block
  (Development|PrintString "BLOCK" true true "(R=0.000000,G=0.660000,B=1.000000,A=1.000000)" 1.0)
  (Variables|Default|SetEnemyMode "NewEnumerator1")
  (Variables|Default|SetPlayerMode "NewEnumerator2")
  (bind _output_get (Variables|Default|SetHP_Player (- (Variables|Default|GetHP_Player) (* (Variables|Default|GetStrength_Enemy) 0.2))))
  (if (<= _output_get 0.0)
    (Variables|Default|SetHP_Player (Math|Random|RandomFloatinRange 5e+01 1e+02))
    (Variables|Default|SetPlayerMode "NewEnumerator3")
    (else
      (bind _output_get_2 (Variables|Default|SetHP_Enemy (- (Variables|Default|GetHP_Enemy) (* (Variables|Default|GetStrength_Player) 0.5))))
      (if (<= _output_get_2 0.0)
        (Variables|Default|SetEnemyMode "NewEnumerator3")))))

(fn Run
  (Development|PrintString "RUN" true true "(R=0.000000,G=0.660000,B=1.000000,A=1.000000)" 1.0)
  (Variables|Default|SetPlayerMode "NewEnumerator0")
  (Variables|Default|SetEnemyMode "NewEnumerator0")
  (bind _output_get (Variables|Default|SetHP_Enemy (Math|Random|RandomFloatinRange 5e+01 1e+02)))
  (Variables|Default|SetHP_EnemyInit _output_get)
  (Variables|Default|SetHP_Player (+ (Variables|Default|GetHP_Player) 1e+01)))

(fn SetAnimationPlayer
  (params (NewParam :type AnimationEnum%20Enum :default "NewEnumerator0"))
  (switch Utilities|FlowControl|Switch|SwitchonAnimationEnum NewParam
    (:NewEnumerator0
      (Sprite|SetFlipbook (Variables|Default|GetPlayerFlipbook) "/Game/Sprites/Cultist/Walk/Idle.Idle")
      (Components|Timeline|SetLooping (Variables|Default|GetPlayerFlipbook) false)
      (Audio|Components|Audio|Play (Variables|Default|GetPlayerFlipbook)))
    (:NewEnumerator1
      (Sprite|SetFlipbook (Variables|Default|GetPlayerFlipbook) "/Game/Sprites/Cultist/Attack/Attack1.Attack1")
      (Components|Timeline|SetLooping (Variables|Default|GetPlayerFlipbook) false)
      (Audio|Components|Audio|Play (Variables|Default|GetPlayerFlipbook)))
    (:NewEnumerator2
      (Sprite|SetFlipbook (Variables|Default|GetPlayerFlipbook) "/Game/Sprites/Cultist/Block/BlockBegin.BlockBegin")
      (Components|Timeline|SetLooping (Variables|Default|GetPlayerFlipbook) false)
      (Audio|Components|Audio|Play (Variables|Default|GetPlayerFlipbook)))
    (:NewEnumerator3
      (Sprite|SetFlipbook (Variables|Default|GetPlayerFlipbook) "/Game/Sprites/Cultist/Death/Death1.Death1")
      (Components|Timeline|SetLooping (Variables|Default|GetPlayerFlipbook) false)
      (Audio|Components|Audio|Play (Variables|Default|GetPlayerFlipbook)))))

(fn SetAnimationEnemy
  (params (NewParam :type AnimationEnum%20Enum :default "NewEnumerator0"))
  (switch Utilities|FlowControl|Switch|SwitchonAnimationEnum NewParam
    (:NewEnumerator0
      (Sprite|SetFlipbook (Variables|Default|GetEnemyFlipbook) "/Game/Sprites/Cultist/Walk/Idle.Idle")
      (Components|Timeline|SetLooping (Variables|Default|GetEnemyFlipbook) true)
      (Audio|Components|Audio|Play (Variables|Default|GetEnemyFlipbook)))
    (:NewEnumerator1
      (Sprite|SetFlipbook (Variables|Default|GetEnemyFlipbook) "/Game/Sprites/Cultist/Attack/Attack1.Attack1")
      (Components|Timeline|SetLooping (Variables|Default|GetEnemyFlipbook) false)
      (Audio|Components|Audio|Play (Variables|Default|GetEnemyFlipbook)))
    (:NewEnumerator2
      (Sprite|SetFlipbook (Variables|Default|GetEnemyFlipbook) "/Game/Sprites/Cultist/Block/BlockBegin.BlockBegin")
      (Components|Timeline|SetLooping (Variables|Default|GetEnemyFlipbook) false)
      (Components|Timeline|PlayfromStart (Variables|Default|GetEnemyFlipbook)))
    (:NewEnumerator3
      (Sprite|SetFlipbook (Variables|Default|GetEnemyFlipbook) "/Game/Sprites/Cultist/Death/Death1.Death1")
      (Components|Timeline|SetLooping (Variables|Default|GetEnemyFlipbook) false)
      (Audio|Components|Audio|Play (Variables|Default|GetEnemyFlipbook)))))